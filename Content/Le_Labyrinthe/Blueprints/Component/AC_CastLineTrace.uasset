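; AC_CastLineTrace is an interaction component for Le_Labyrinthe that lets the player light a torch or unlock a lever they look at.
; CastLineTrace fires a short line trace along the player camera's forward vector, with debug drawing on.
; It matches the hit component's name against "Torch" or "Lever", then calls Lit or Unlocked on the actor GetActorOfClass returns for BP_Torche or BP_Lever, rather than on the hit actor.
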(event Custom|CastLineTrace
  (bind _returnvalue (Game|GetPlayerCameraManager 0))
  (bind _rootcomponent (Variables|/Script/Engine.Actor|GetRootComponent _returnvalue))
  (bind _returnvalue_2 (Transformation|GetWorldLocation _rootcomponent))
  ;[1 1 1] Find where the line trace should start and end .
  ;[1 1 1] Cast trace and Making the component hit work if possible
  (bind _outhit (Collision|LineTraceByChannel _returnvalue_2 (+ _returnvalue_2 (* (Transformation|GetActorForwardVector _returnvalue) 5e+02)) "TraceTypeQuery3" false 0 "ForDuration"))
  ;;[1 1 1] Torch
  (if (Utilities|Enum|Equal(Enum) (Utilities|GetObjectName (.HitComponent (Collision|BreakHitResult _outhit))) "Torch")
    (bind _returnvalue_3 (Actor|GetActorOfClass "/Game/Le_Labyrinthe/Blueprints/BP_Torche.BP_Torche_C"))
    (Default|Lit _returnvalue_3)
    (else
      ;;[1 1 1] Comment
      (if (Utilities|Enum|Equal(Enum) (Utilities|GetObjectName (.HitComponent (Collision|BreakHitResult _outhit))) "Lever")
        (bind _returnvalue_4 (Actor|GetActorOfClass "/Game/Le_Labyrinthe/Blueprints/BP_Lever.BP_Lever_C"))
        (Default|Unlocked _returnvalue_4)))))