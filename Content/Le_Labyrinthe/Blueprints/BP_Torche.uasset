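; BP_Torche is a toggleable torch in the labyrinth that works with a lever to control a secret door.
; The Lit event toggles the PFire effect and IsLit state.
; Lighting rotates the Secret actor to unlock it if the BP_Lever found in the level is unlocked.
; Extinguishing is meant to relock it, but rotates the torch itself when Secret is at its open rotation.
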(event Custom|Lit
  (bind _p_fire (Variables|Default|GetP_Fire))
  ;[1 1 1] lit or unlit the torch
  (if (Variables|Default|GetIsLit)
    (Components|Activation|Deactivate _p_fire)
    (Variables|Default|SetIsLit false)
    ;[1 1 1] If you kill the torch flame the door should go back to be locked
    (if (Utilities|Operators|EqualEqual (Transformation|GetActorRotation (Variables|Default|GetSecret)) "0.000000,90.000000,0.000000" 0.0)
      (Transformation|SetActorRotation "0.000000,-90.000000,0.000000"))
    (else
      (Components|Activation|Activate _p_fire false)
      (Variables|Default|SetIsLit true)
      ;[1 1 1] If the lever has been used then unlock the door
      (bind _returnvalue (Actor|GetActorOfClass "/Game/Le_Labyrinthe/Blueprints/BP_Lever.BP_Lever_C"))
      (if (not (Variables|/Game/Le_Labyrinthe/Blueprints/BP_Lever.BP_Lever_C|GetIsLocked _returnvalue))
        (Transformation|SetActorRotation (Variables|Default|GetSecret) "0.000000,90.000000,0.000000")))))

(fn ConstructionScript)