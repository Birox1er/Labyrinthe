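; Player controller for the labyrinth game that turns Enhanced Input actions into first-person movement, camera look and activation.
; On BeginPlay it adds the player controls mapping context, then applies camera input to its own yaw and pitch.
; Movement follows control rotation, and activation calls the character's line trace component.
; Both reach BP_FirstPersonCharacter through GetActorOfClass on each trigger rather than through the possessed pawn.
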(event Input|EnhancedActionEvents|EnhancedInputActionIA_Movement
  (params (ActionValue :type Vector%202D%20Structure) (ElapsedSeconds :type Float%20%28double-precision%29) (TriggeredSeconds :type Float%20%28double-precision%29) (InputAction :type Input%20Action%20Object%20Reference :default "/Game/Le_Labyrinthe/Input/InputAction/IA_Movement.IA_Movement"))
  (bind _returnvalue (Pawn|GetControlRotation :!class /Script/Engine.Controller))
  ;[1 1 1] Movement
  (:Triggered
    (bind _returnvalue_2 (Actor|GetActorOfClass "/Game/Le_Labyrinthe/Blueprints/BP_FirstPersonCharacter.BP_FirstPersonCharacter_C"))
    (Pawn|Input|AddMovementInput _returnvalue_2 (Math|Vector|GetRightVector (Math|Rotator|MakeRotator (.roll _returnvalue) 0.0 (.yaw _returnvalue))) (.x ActionValue) false)
    (Pawn|Input|AddMovementInput _returnvalue_2 (Math|Vector|GetForwardVector (Math|Rotator|MakeRotator 0.0 0.0 (.yaw _returnvalue))) (.y ActionValue) false)))

(event Input|EnhancedActionEvents|EnhancedInputActionIA_Camera
  (params (ActionValue :type Vector%202D%20Structure) (ElapsedSeconds :type Float%20%28double-precision%29) (TriggeredSeconds :type Float%20%28double-precision%29) (InputAction :type Input%20Action%20Object%20Reference :default "/Game/Le_Labyrinthe/Input/InputAction/IA_Camera.IA_Camera"))
  ;[1 1 1] Camera control
  (:Triggered
    (Class|PlayerController|AddYawInput (.x ActionValue))
    (Class|PlayerController|AddPitchInput (.y ActionValue))))

(event Input|EnhancedActionEvents|EnhancedInputActionIA_Activation
  (params (ActionValue :type Boolean) (ElapsedSeconds :type Float%20%28double-precision%29) (TriggeredSeconds :type Float%20%28double-precision%29) (InputAction :type Input%20Action%20Object%20Reference :default "/Game/Le_Labyrinthe/Input/InputAction/IA_Activation.IA_Activation"))
  ;[1 1 1] Cast LineTrace
  (:Triggered
    (bind _returnvalue (Actor|GetActorOfClass "/Game/Le_Labyrinthe/Blueprints/BP_FirstPersonCharacter.BP_FirstPersonCharacter_C"))
    (Default|CastLineTrace (Variables|/Game/Le_Labyrinthe/Blueprints/BP_FirstPersonCharacter.BP_FirstPersonCharacter_C|GetAC_CastLineTrace _returnvalue))))

(event EventBeginPlay
  (bind _self self)
  (bind _returnvalue (PlayerController|LocalPlayerSubsystems|GetEnhancedInputLocalPlayerSubsystem _self))
  ;[1 1 1] Setting up mapping contexts
  (Utilities|IsValid _returnvalue
    (:Is%20Valid
      (Utilities|String|LogString "Hello")
      (Input|AddMappingContext _returnvalue "/Game/Le_Labyrinthe/Input/IMC_PlayerControls.IMC_PlayerControls" 0 "(bIgnoreAllPressedKeysUntilRelease=True,bForceImmediately=False)"))))

(fn ConstructionScript)